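; BP_ObjectPool_Be is an object pool that pre-spawns PoolSize actors of ActorClass at BeginPlay and deactivates them for reuse.
; ActorPool maps each actor to an in-use flag, which ReturnActor clears before deactivating the actor.
; GetActor linearly scans for a free actor, activates it and calls ResetMessage, or spawns a new one when none is free, so the pool grows on demand.
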(event `self.ReceiveBeginPlay`
  ;[1 1 1] InitPool
  (for _ (range (+ (`self.PoolSize`) 1))
    (`self.CreateNewActor`)))

(fn `CreateNewActor`
  (returns (NewActor :type "Actor Object Reference"))
  (bind _returnvalue (`|SpawnActorFromClass` (`self.ActorClass`) (`KismetMathLibrary.MakeTransform` (0.0 0.0 0.0)) "AlwaysSpawn" "OverrideRootScale" self null))
  (`BlueprintMapLibrary.Map_Add` (`self.ActorPool`) _returnvalue)
  (`/Game/Core/FunctionLibrary_Be.DeactivateActor` _returnvalue)
  (return _returnvalue))

(fn `GetActor`
  (returns (Actor :type "Actor Object Reference"))
  (bind _actorpool (`self.ActorPool`))
  (bind _values (`BlueprintMapLibrary.Map_Values` (`self.ActorPool`)))
  (for (_array_element _array_index) _values
    (if (not _array_element)
      (bind _keys (`BlueprintMapLibrary.Map_Keys` _actorpool))
      (bind _output (`|GetArrayItem` _keys _array_index))
      (`/Game/Core/FunctionLibrary_Be.ActivateActor` _output)
      (`BlueprintMapLibrary.Map_Add` _actorpool _output true)
      (message `/Game/Core/PoolingInterface_Be.Reset` _output)
      (`KismetSystemLibrary.PrintString` (`KismetSystemLibrary.GetDisplayName` _output))
      (return _output)))
  (bind _newactor (`self.CreateNewActor`))
  (`/Game/Core/FunctionLibrary_Be.ActivateActor` _newactor)
  (`BlueprintMapLibrary.Map_Add` (`self.ActorPool`) _newactor true)
  (return _newactor))

(fn `ReturnActor`
  (params (Actor :type "Actor Object Reference"))
  (`BlueprintMapLibrary.Map_Add` (`self.ActorPool`) Actor)
  (`/Game/Core/FunctionLibrary_Be.DeactivateActor` Actor))

(fn `UserConstructionScript`)