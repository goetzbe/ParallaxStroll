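; Component on the 2D side-scroller character that projects world objects onto the player's Y=0 plane.
; BeginPlay caches every BPI_ProjectableInterface_Be actor.
; ProjectObjects intersects the camera ray through each recently rendered actor's object-pane sprite with that plane, moves the player-pane sprite there and scales it by the intercept theorem to preserve perspective.
; CollisionProjection is an empty stub; Tick and object-pane rescaling are inactive.
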(event `self.ReceiveBeginPlay`
  ;[1 1 1] Get all objects to project
  (bind _outactors (`GameplayStatics.GetAllActorsWithInterface` "/Game/Core/BPI_ProjectableInterface_Be.BPI_ProjectableInterface_Be_C"))
  (bind _output_get (set `self.toProject` _outactors)))

(event `ProjectObjects`
  (bind (_cameralocation_x _cameralocation_y) (`KismetMathLibrary.BreakVector` (`self.CameraLocation`)))
  (bind _returnvalue (- (`self.ObjectPaneLocation`) (`self.CameraLocation`)))
  (bind _returnvalue_2 (+ (* _returnvalue (/ (* _cameralocation_y -1.0) (.y _returnvalue))) (`self.CameraLocation`)))
  ;[1 1 1] PlayerPlaneProjection (PPP)
  ;;[1 1 1] for each actor to project
  (for (_array_element _array_index) (`self.toProject`)
    ;;[1 1 1] only display actors on screen
    (if (`Actor.WasRecentlyRendered` _array_element 0.2)
      (bind _objectpanesprite (message `/Game/Core/BPI_ProjectableInterface_Be.GetObjectPaneSprite` _array_element))
      (set `self.ObjectPaneLocation` (`SceneComponent.K2_GetComponentLocation` _objectpanesprite))
      (set `self.CameraLocation` (`SceneComponent.K2_GetComponentLocation` (`/Game/Characters/Player/BP_2DSideScrollerCharacter_Be.SideViewCameraComponent` (cast `/Game/Characters/Player/BP_2DSideScrollerCharacter_Be` (`self.GetOwner`) :!pure true))))
      ;;[1 1 1] adjust to new location (through syncing centres)
      (bind _playerpanesprite (message `/Game/Core/BPI_ProjectableInterface_Be.GetPlayerPaneSprite` _array_element))
      (`SceneComponent.K2_AddRelativeLocation` _playerpanesprite (- _returnvalue_2 (`SceneComponent.K2_GetComponentLocation` _playerpanesprite)) false false)
      (bind _relativescale3d_x (`KismetMathLibrary.BreakVector` (`SceneComponent.RelativeScale3D` _objectpanesprite)))
      (bind _returnvalue_3 (* _relativescale3d_x (/ (`KismetMathLibrary.VSize` (- _returnvalue_2 (`self.CameraLocation`))) (`KismetMathLibrary.VSize` _returnvalue))))
      ;;[1 1 1] Adjust scale
      (`SceneComponent.SetRelativeScale3D` _playerpanesprite (`KismetMathLibrary.MakeVector` _returnvalue_3 1.0 _returnvalue_3)))))

(event `CollisionProjection`
  ;[1 1 1] for each actor to project
  (for _array_element (`self.toProject`)
    ;[1 1 1] only display actors on screen
    (if (`Actor.WasRecentlyRendered` _array_element 0.2)
      _)))

(fn `Compute Intersection Line Player Plane`
  (params (SupportVector :type "Vector Structure") (DirectionReferencePoint :type "Vector Structure"))
  (returns (IntersectionPoint :type "Vector Structure"))
  (bind _returnvalue (- DirectionReferencePoint SupportVector))
  (bind (_cameralocation_x _cameralocation_y) (`KismetMathLibrary.BreakVector` (`self.CameraLocation`)))
  (return (+ (* _returnvalue (/ (* _cameralocation_y -1.0) (.y _returnvalue))) (`self.CameraLocation`))))