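; Color-reactive trap that damages a side-scroller character on overlap while active.
; On BeginPlay it sets the spline's child box components to overlap all channels and registers with the player AnneDroid's ColorObserver for three events, repeating the registration per box.
; Trigger deactivates and hides the trap when the event index matches ReactToEvent, and reactivates and shows it for any other index.
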(event `self.ReceiveBeginPlay`
  (bind _colorobserver (`/Game/Characters/Player/BP_AnneDroid_Be.ColorObserver` (cast `/Game/Characters/Player/BP_AnneDroid_Be` (`GameplayStatics.GetPlayerCharacter` 0) :!pure true)))
  (`parent.ReceiveBeginPlay`)
  (for _array_element (`SceneComponent.GetChildrenComponents` (`self.Spline`) false)
    (bind _asbox_collision (cast `BoxComponent` _array_element))
    (`PrimitiveComponent.SetCollisionResponseToAllChannels` _asbox_collision "ECR_Overlap")
    (`/Game/Core/ColorSwitch/Observer.RegisterForEvent` _colorobserver 0 self)
    (`/Game/Core/ColorSwitch/Observer.RegisterForEvent` _colorobserver 1 self)
    (`/Game/Core/ColorSwitch/Observer.RegisterForEvent` _colorobserver 2 self)))

(event `self.ReceiveActorBeginOverlap`
  (params (OtherActor :type "Actor Object Reference"))
  ;[1 1 1] Apply damage on hit
  (if (`self.Active`)
    (`KismetSystemLibrary.PrintString` "overlapped")
    (bind _asside_scroller_character (cast `/Game/Characters/Player/SideScrollerCharacter` OtherActor))
    (`GameplayStatics.ApplyDamage` _asside_scroller_character (`self.Damage`) (`self.GetInstigatorController`) self "/Script/Engine.DamageType")
    (`KismetSystemLibrary.PrintString` "Damaged")))

(event `/Game/Core/ColorSwitch/Triggerable.Trigger`
  (params (Index :type Integer))
  (bind _output_get (set `self.Active` (!= Index (`self.ReactToEvent`))))
  (`self.SetActorHiddenInGame` (not _output_get)))

(fn `UserConstructionScript`)