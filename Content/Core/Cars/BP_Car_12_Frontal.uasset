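; Car actor for a side-scroller whose spline outline is projected from the side-view camera's perspective onto the player plane (Y=0) as a chain of box components.
; BeginPlay adds one box per spline segment, closing the loop.
; While recently rendered, Tick intersects camera-to-spline-point rays with that plane, then moves, rotates and scales each box to join neighboring projected points, so the boxes follow the outline's on-screen shape.
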(event `self.ReceiveBeginPlay`
  (bind _spline (`self.Spline`))
  (bind _returnvalue (`SplineComponent.GetNumberOfSplinePoints` (`self.Spline`)))
  ;[1 1 1] Initialization
  (set `self.ProjectionCamera` (`/Game/Characters/Player/SideScrollerCharacter.SideViewCamera` (cast `/Game/Characters/Player/SideScrollerCharacter` (`GameplayStatics.GetPlayerCharacter` 0) :!pure true)))
  (for _index (range _returnvalue)
    (bind _returnvalue_2 (`AddComponent|NODE_AddBoxComponent-1`))
    (`SceneComponent.K2_AttachToComponent` _returnvalue_2 (`self.Spline`) "None" "KeepRelative" "KeepRelative" "KeepRelative" true)
    (bind _returnvalue_3 (`SplineComponent.GetLocationAtSplinePoint` _spline _index "World"))
    (bind _returnvalue_4 (- (`SplineComponent.GetLocationAtSplinePoint` _spline (mod (+ _index 1) _returnvalue) "World") _returnvalue_3))
    (`SceneComponent.SetWorldScale3D` _returnvalue_2 (`KismetMathLibrary.MakeVector` (* (`KismetMathLibrary.VSize` _returnvalue_4) 0.5) 1.0 1.0))
    (bind _z (.z _returnvalue_4))
    (bind _angle (`self.AngleBetweenTwoVectors` (`KismetMathLibrary.MakeVector` (.x _returnvalue_4) 0.0 _z) (1.0 0.0 0.0)))
    (bind (_returnvalue_x _returnvalue_y _returnvalue_z) (`KismetMathLibrary.BreakVector` (+ _returnvalue_3 (* _returnvalue_4 0.5))))
    (`SceneComponent.K2_SetWorldLocationAndRotation` _returnvalue_2 (`KismetMathLibrary.MakeVector` _returnvalue_x 0.0 _returnvalue_z) (`KismetMathLibrary.MakeRotator` 0.0 (select `bool` (< _z 0.0) :`false` _angle :`true` (- 360.0 _angle))) false false)
    (`KismetArrayLibrary.Array_Add` (`self.ProjectedPoints`) _returnvalue_3)))

(event `self.ReceiveTick`
  (params (DeltaSeconds :type "Float (single-precision)"))
  (bind _returnvalue (`SplineComponent.GetNumberOfSplinePoints` (`self.Spline`)))
  ;[1 1 1] PlayerPlaneProjection (PPP)
  ;;[1 1 1] only display actors on screen
  (if (`self.WasRecentlyRendered` 0.2)
    (bind _output_get (set `self.CameraLocation` (`SceneComponent.K2_GetComponentLocation` (`self.ProjectionCamera`))))
    (for _index (range _returnvalue)
      (bind _intersectionpoint (`self.ComputeIntersectionLinePlayerPlane` _output_get (`SplineComponent.GetLocationAtSplinePoint` (`self.Spline`) _index "World")))
      (`KismetArrayLibrary.Array_Set` (`self.ProjectedPoints`) _index _intersectionpoint))
    (for (_array_element _array_index) (`SceneComponent.GetChildrenComponents` (`self.Spline`) false)
      (bind _output (`|GetArrayItem` (`self.ProjectedPoints`) _array_index))
      (bind _returnvalue_2 (- (`|GetArrayItem` (`self.ProjectedPoints`) (mod (+ _array_index 1) _returnvalue)) _output))
      (`SceneComponent.SetWorldScale3D` _array_element (`KismetMathLibrary.MakeVector` (* (`KismetMathLibrary.VSize` _returnvalue_2) 0.5) 1.0 1.0))
      (bind _angle (`self.AngleBetweenTwoVectors` _returnvalue_2 (1.0 0.0 0.0)))
      (`SceneComponent.K2_SetWorldLocationAndRotation` _array_element (+ _output (* _returnvalue_2 0.5)) (`KismetMathLibrary.MakeRotator` 0.0 (select `bool` (< (.z _returnvalue_2) 0.0) :`false` _angle :`true` (- 360.0 _angle))) false false))))

(fn `AngleBetweenTwoVectors`
  (params (A :type "Vector Structure") (B :type "Vector Structure"))
  (returns (Angle :type "Float (double-precision)"))
  ;[1 1 1] Angle between two vectors
  (return (`KismetMathLibrary.DegAcos` (`KismetMathLibrary.Dot_VectorVector` (`KismetMathLibrary.Normal` A) (`KismetMathLibrary.Normal` B)))))

(fn `ComputeIntersectionLinePlayerPlane`
  (params (SupportVector :type "Vector Structure") (DirectionReferencePoint :type "Vector Structure"))
  (returns (IntersectionPoint :type "Vector Structure"))
  (bind _returnvalue (- DirectionReferencePoint SupportVector))
  (bind (_cameralocation_x _cameralocation_y) (`KismetMathLibrary.BreakVector` (`self.CameraLocation`)))
  (return (+ (* _returnvalue (/ (* _cameralocation_y -1.0) (.y _returnvalue))) (`self.CameraLocation`))))

(fn `UserConstructionScript`)