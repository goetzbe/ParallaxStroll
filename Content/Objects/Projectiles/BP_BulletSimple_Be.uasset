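; Simple bullet projectile that damages a SideScrollerCharacter when its static mesh hits one.
; Any mesh hit prints a debug message and sets a near-zero lifespan, then a successful character cast applies damage credited to the instigator's controller.
; An unconnected leftover loop would set box components under a spline to block all channels, but it never runs.
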(event `self.ReceiveBeginPlay`
  (`parent.ReceiveBeginPlay`))

(event `self.StaticMesh.OnComponentHit`
  (params (HitComponent :type "PrimitiveComponent Object Reference") (OtherActor :type "Actor Object Reference") (OtherComp :type "PrimitiveComponent Object Reference") (NormalImpulse :type "Vector Structure") (Hit :type "HitResult Structure (by ref)"))
  (`KismetSystemLibrary.PrintString` "mesh hit")
  (`self.SetLifeSpan` 0.01)
  (bind _asside_scroller_character (cast `/Game/Characters/Player/SideScrollerCharacter` OtherActor))
  (`GameplayStatics.ApplyDamage` _asside_scroller_character (`self.Damage`) (`self.GetInstigatorController`) self "/Script/Engine.DamageType"))

(fn `UserConstructionScript`
  (`parent.UserConstructionScript`))