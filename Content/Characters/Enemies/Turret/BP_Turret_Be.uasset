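; Enemy turret that tracks the closest visible Character in sensing range and shoots pooled bullets at it.
; Each tick it caps the base mesh's upward velocity, picks a target by sphere overlap and line of sight, and turns the top mesh at constant speed within pitch/yaw limits.
; When aligned and off cooldown, it launches a bullet from the left barrel socket, using the object pool tagged "Bullets" found at BeginPlay.
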(event `self.ReceiveTick`
  (params (DeltaSeconds :type "Float (single-precision)"))
  (bind (_returnvalue_x _returnvalue_y _returnvalue_z) (`KismetMathLibrary.BreakVector` (`self.GetVelocity`)))
  (`PrimitiveComponent.SetPhysicsLinearVelocity` (`self.StaticMeshBase`) (`KismetMathLibrary.MakeVector` _returnvalue_x _returnvalue_y (`KismetMathLibrary.FClamp` _returnvalue_z _returnvalue_z (`self.MaxZSpeed`))) false "None")
  (`self.FindBestTarget`)
  (`self.Target`
    (:`then`
      (`self.UpdateTurretRotation` DeltaSeconds)
      (`self.UpdateFire`))
    (:`else`)))

(event `Fire`
  (bind (_returnvalue_location _returnvalue_rotation) (`KismetMathLibrary.BreakTransform` (`SceneComponent.GetSocketTransform` (`self.StaticMeshLeftBarrel`) "FireSocket" "RTS_World")))
  (set `self.TimeOfLastShot` (`KismetSystemLibrary.GetGameTimeInSeconds`))
  (`|ExecutionSequence`
    (:`then_0`
      (goto _label :!via `Reset`))
    (:`then_1`
      (`/Engine/EditorBlueprintResources/StandardMacros.Do N` 1 :!label _label
        (:`Exit`
          (bind _actor (`/Game/Core/BP_ObjectPool_Be.GetActor` (`self.BulletPool`)))
          (`self.K2_SetActorTransform` _actor (`KismetMathLibrary.MakeTransform` _returnvalue_location _returnvalue_rotation (0.15 0.15 0.15)) false false)
          (bind _asbp_bullet_projected_be (cast `/Game/Objects/Projectiles/BP_BulletProjected_Be` _actor))
          (`/Game/Objects/Projectiles/BP_BulletProjected_Be.LaunchProjectile` _asbp_bullet_projected_be false (* (`KismetMathLibrary.GetForwardVector` _returnvalue_rotation) 500.0)))))))

(event `self.ReceiveBeginPlay`
  (bind _outactors (`GameplayStatics.GetAllActorsOfClassWithTag` "/Game/Core/BP_ObjectPool_Be.BP_ObjectPool_Be_C" "Bullets"))
  (set `self.BulletPool` (`|GetArrayItem` _outactors)))

(fn `FindBestTarget`
  (locals (`BestDistance (local)` :type "Float (double-precision)") (`CurrentDistance (local)` :type "Float (double-precision)") (`BestTarget (local)` :type "Actor Object Reference") (`CurrentTarget (local)` :type "Actor Object Reference"))
  (set `local.BestDistance (local)` (+ (`self.SensingRange`) 1.0))
  (bind _outactors (`KismetSystemLibrary.SphereOverlapActors` (`self.K2_GetActorLocation`) (`self.SensingRange`) (`|MakeArray` "ObjectTypeQuery3" :!type "EObjectTypeQuery Enum") "/Script/Engine.Character"))
  (for _array_element _outactors
    (bind _output_get (set `local.CurrentTarget (local)` _array_element))
    (bind _output_get_2 (set `local.CurrentDistance (local)` (`self.GetDistanceTo` _output_get self)))
    (if (or (< _output_get_2 (`local.BestDistance (local)`)) (not (`KismetSystemLibrary.IsValid` (`local.BestTarget (local)`))))
      (bind _result (`/Game/Core/FunctionLibrary_Be.HasLineOfSight` (`SceneComponent.K2_GetComponentLocation` (`self.StaticMeshTop`)) (`self.K2_GetActorLocation` (`local.CurrentTarget (local)`)) (`|MakeArray` self (`local.CurrentTarget (local)`) :!type "Actor Object Reference")))
      (if _result
        (set `local.BestTarget (local)` (`local.CurrentTarget (local)`))
        (set `local.BestDistance (local)` (`local.CurrentDistance (local)`)))))
  (set `self.Target` (`local.BestTarget (local)`)))

(fn `UpdateFire`
  (if (> (- (`KismetSystemLibrary.GetGameTimeInSeconds`) (`self.TimeOfLastShot`)) (`self.RateOfFire`))
    (if (> (`KismetMathLibrary.Dot_VectorVector` (`KismetMathLibrary.GetDirectionUnitVector` (`SceneComponent.K2_GetComponentLocation` (`self.StaticMeshTop`)) (`self.K2_GetActorLocation` (`self.Target`))) (`SceneComponent.GetForwardVector` (`self.StaticMeshTop`))) 0.99)
      (`self.Fire`))))

(fn `UpdateTurretRotation`
  (params (DeltaSeconds :type "Float (double-precision)"))
  (locals (`NewRotation (local)` :type "Rotator Structure" :default (struct)))
  (bind _output_get (set `local.NewRotation (local)` (`KismetMathLibrary.RInterpTo_Constant` (`SceneComponent.K2_GetComponentRotation` (`self.StaticMeshTop`)) (`KismetMathLibrary.FindLookAtRotation` (`SceneComponent.K2_GetComponentLocation` (`self.StaticMeshTop`)) (`self.K2_GetActorLocation` (`self.Target`))) (`local.DeltaSeconds`) (`self.RotationSpeed`))))
  (`SceneComponent.K2_SetWorldRotation` (`self.StaticMeshTop`) (`KismetMathLibrary.MakeRotator` (.roll _output_get) (`KismetMathLibrary.ClampAngle` (.pitch _output_get) -45.0 75.0) (`KismetMathLibrary.ClampAngle` (.yaw _output_get) 90.0 270.0)) false false))

(fn `UserConstructionScript`)