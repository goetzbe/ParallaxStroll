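; BP_AnneDroid_Be is a player character Blueprint that adds number-key toggles for changing the scene's color mood.
; On BeginPlay, after calling its parent, it caches every DirectionalLight in the level.
; Keys 1 and 2 recolor those lights warm or pure blue.
; Keys 3 and 4 swap the SideViewCamera's entire post-process settings between the BlueTint and NoTint presets.
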(event `self.ReceiveBeginPlay`
  (`parent.ReceiveBeginPlay`)
  (bind _outactors (`GameplayStatics.GetAllActorsOfClass` "/Script/Engine.DirectionalLight"))
  (set `self.LightsColors` _outactors))

(event `Key|Two`
  (params (Key :type "Key Structure"))
  (:`Pressed`
    (for _array_element (`self.LightsColors`)
      (`LightComponent.SetLightColor` (`Light.LightComponent` _array_element) (struct :`B` 1.0 :`A` 1.0) true))))

(event `Key|One`
  (params (Key :type "Key Structure"))
  (:`Pressed`
    (for _array_element (`self.LightsColors`)
      (`LightComponent.SetLightColor` (`Light.LightComponent` _array_element) (struct :`R` 1.0 :`G` 0.807843 :`B` 0.603922 :`A` 1.0) true))))

(event `Key|Four`
  (params (Key :type "Key Structure"))
  (:`Pressed`
    (set `CameraComponent.PostProcessSettings` (`self.NoTint`) (`self.SideViewCamera`))))

(event `Key|Three`
  (params (Key :type "Key Structure"))
  (:`Pressed`
    (set `CameraComponent.PostProcessSettings` (`self.BlueTint`) (`self.SideViewCamera`))))

(fn `UserConstructionScript`
  (`parent.UserConstructionScript`))