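; Pooled bullet projectile that damages any SideScrollerCharacter it hits.
; It starts stationary, and launch and stop events set its ProjectileMovement velocity, with launches in local or world space.
; Tick counts down a lifespan, which a hit zeroes, and returns the expired bullet to its owning BP_ObjectPool_Be instead of destroying it.
; Reset restores the lifespan and reattaches the movement component to the mesh for reuse.
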(event `self.ReceiveTick`
  (params (DeltaSeconds :type "Float (single-precision)"))
  ;[1 1 1] Return bullet to pool, if life span is 0
  (`parent.ReceiveTick` DeltaSeconds)
  (bind _output_get (set `self.CurrentLifeSpan` (- (`self.CurrentLifeSpan`) DeltaSeconds)))
  (if (<= _output_get 0.0)
    (bind _asbp_object_pool_be (cast `/Game/Core/BP_ObjectPool_Be` (`self.GetOwner`)))
    (`/Game/Core/BP_ObjectPool_Be.ReturnActor` _asbp_object_pool_be self)))

(event `self.ReceiveBeginPlay`
  ;[1 1 1] Stop projectile at start
  (`self.StopProjectile`)
  (`parent.ReceiveBeginPlay`))

(event `self.StaticMesh.OnComponentHit`
  (params (HitComponent :type "PrimitiveComponent Object Reference") (OtherActor :type "Actor Object Reference") (OtherComp :type "PrimitiveComponent Object Reference") (NormalImpulse :type "Vector Structure") (Hit :type "HitResult Structure (by ref)"))
  ;[1 1 1] Apply damage on hit
  (set `self.CurrentLifeSpan` 0.0)
  (bind _asside_scroller_character (cast `/Game/Characters/Player/SideScrollerCharacter` OtherActor))
  (`GameplayStatics.ApplyDamage` _asside_scroller_character (`self.Damage`) (`self.GetInstigatorController`) self "/Script/Engine.DamageType"))

(event `/Game/Core/PoolingInterface_Be.Reset`
  ;[1 1 1] Reset bullet
  (set `self.CurrentLifeSpan` (`self.MaxLifeSpan`))
  (`MovementComponent.SetUpdatedComponent` (`self.ProjectileMovement`) (`self.StaticMesh`)))

(event `LaunchProjectile`
  (params (`Launch in local space?` :type Boolean) (`Launch veloctiy` :type "Vector Structure"))
  ;[1 1 1] Launch projectile
  (if `Launch in local space?`
    (`ProjectileMovementComponent.SetVelocityInLocalSpace` (`self.ProjectileMovement`) `Launch veloctiy`)
    (else
      (set `MovementComponent.Velocity` `Launch veloctiy` (`self.ProjectileMovement`)))))

(event `StopProjectile`
  ;[1 1 1] Stop projectile
  (`ProjectileMovementComponent.SetVelocityInLocalSpace` (`self.ProjectileMovement`) (0.0 0.0 0.0)))

(fn `UserConstructionScript`
  (`parent.UserConstructionScript`))